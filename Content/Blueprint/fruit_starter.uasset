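; Fruit actor that starts the game when a katana touches it.
; The construction script copies its static mesh into a procedural mesh with collision.
; When its sphere overlaps a katana, it enables gravity on that mesh and calls StartGame on the Launcher and StartSpecial on Launcher_2.
; A delayed self-destroy branch exists but is not connected, so it never runs.
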(event `self.ReceiveBeginPlay`)

(event `self.Sphere.OnComponentBeginOverlap`
  (params (OverlappedComponent :type "PrimitiveComponent Object Reference") (OtherActor :type "Actor Object Reference") (OtherComp :type "PrimitiveComponent Object Reference") (OtherBodyIndex :type Integer) (bFromSweep :type Boolean) (SweepResult :type "HitResult Structure (by ref)"))
  (cast `/Game/blueprints/katana` OtherActor)
  (`PrimitiveComponent.SetEnableGravity` (`self.ProceduralMesh`) true)
  (bind _returnvalue (`GameplayStatics.GetActorOfClass` "/Game/blueprints/Launcher.Launcher_C"))
  (`/Game/blueprints/Launcher.StartGame` _returnvalue)
  (bind _returnvalue_2 (`GameplayStatics.GetActorOfClass` "/Game/blueprints/Launcher_2.Launcher_2_C"))
  (`/Game/blueprints/Launcher_2.StartSpecial` _returnvalue_2))

(fn `UserConstructionScript`
  (`KismetProceduralMeshLibrary.CopyProceduralMeshFromStaticMeshComponent` (`self.StaticMesh`) 0 (`self.ProceduralMesh`) true))
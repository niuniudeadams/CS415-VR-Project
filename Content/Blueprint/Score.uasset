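; Score Blueprint that keeps an integer score and shows it on a text render component in the level.
; BeginPlay writes the initial value to the text render.
; The AddScore event increments the score by one and refreshes the text, formatted to at least four digits without digit grouping.
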(event `Add Score`
  (bind _output_get (set `self.Score` (+ (`self.Score`) 1)))
  (`TextRenderComponent.K2_SetText` (`self.TextRender`) (`KismetTextLibrary.Conv_IntToText` _output_get false false 4)))

(event `self.ReceiveBeginPlay`
  (`TextRenderComponent.K2_SetText` (`self.TextRender`) (`KismetTextLibrary.Conv_IntToText` (`self.Score`) false false 4)))

(fn `UserConstructionScript`)
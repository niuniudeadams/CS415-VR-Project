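; A fruit actor that acts as a hazard for the Katana2 blade, costing health and playing an explosion sound when touched.
; The construction script copies its static mesh into a procedural mesh with collision, and the actor destroys itself three seconds after spawning.
; A sphere overlap lowers Katana2's health, updates its health bar and removes the sphere.
; At zero health it reopens the VRTemplateMap level.
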(event `self.ReceiveBeginPlay`
  (`KismetSystemLibrary.Delay` 3.0)
  (`/Engine/EditorBlueprintResources/StandardMacros.IsValid` (`self.ProceduralMesh`)
    (:`Is Valid`
      (`self.K2_DestroyActor`))))

(event `self.Sphere.OnComponentBeginOverlap`
  (params (OverlappedComponent :type "PrimitiveComponent Object Reference") (OtherActor :type "Actor Object Reference") (OtherComp :type "PrimitiveComponent Object Reference") (OtherBodyIndex :type Integer) (bFromSweep :type Boolean) (SweepResult :type "HitResult Structure (by ref)"))
  (bind _askatana_2 (cast `/Game/Blueprint/Katana2` OtherActor))
  (bind _output_get (set `/Game/Blueprint/Katana2.health` (- (`/Game/Blueprint/Katana2.health` _askatana_2) 50.0) _askatana_2))
  (`/Game/Blueprint/HealthBar.UpdateHealthBar` (`/Game/Blueprint/Katana2.Healthbarreference` _askatana_2) _output_get)
  (`GameplayStatics.PlaySound2D` "/Game/StarterContent/Audio/Explosion01.Explosion01" 1.0 1.0 0.0 null null)
  (`ActorComponent.K2_DestroyComponent` (`self.Sphere`))
  (if (<= _output_get 0.0)
    (`GameplayStatics.OpenLevel` "VRTemplateMap")))

(fn `UserConstructionScript`
  (`KismetProceduralMeshLibrary.CopyProceduralMeshFromStaticMeshComponent` (`self.StaticMesh`) 0 (`self.ProceduralMesh`) true))
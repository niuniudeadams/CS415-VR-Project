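; Special fruit actor that triggers global slow motion when a katana overlaps its Sphere.
; The overlap sets global time dilation very low, restores it after a Delay that itself runs in dilated time, then destroys the fruit.
; The construction script copies the static mesh into a procedural mesh with collision.
; A BeginPlay timeout also destroys the actor after a few seconds if that procedural mesh is valid.
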(event `self.ReceiveBeginPlay`
  (`KismetSystemLibrary.Delay` 3.0)
  (`/Engine/EditorBlueprintResources/StandardMacros.IsValid` (`self.ProceduralMesh`)
    (:`Is Valid`
      (`self.K2_DestroyActor`))))

(event `self.Sphere.OnComponentBeginOverlap`
  (params (OverlappedComponent :type "PrimitiveComponent Object Reference") (OtherActor :type "Actor Object Reference") (OtherComp :type "PrimitiveComponent Object Reference") (OtherBodyIndex :type Integer) (bFromSweep :type Boolean) (SweepResult :type "HitResult Structure (by ref)"))
  (cast `/Game/blueprints/katana` OtherActor)
  (`GameplayStatics.SetGlobalTimeDilation` 0.01)
  (`KismetSystemLibrary.Delay` 0.25)
  (`GameplayStatics.SetGlobalTimeDilation` 1.0)
  (`self.K2_DestroyActor`))

(fn `UserConstructionScript`
  (`KismetProceduralMeshLibrary.CopyProceduralMeshFromStaticMeshComponent` (`self.StaticMesh`) 0 (`self.ProceduralMesh`) true))
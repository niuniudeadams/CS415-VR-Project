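; A fruit target Blueprint that awards score when a Katana2 actor hits it.
; Its construction script copies the static mesh into a procedural mesh with collision.
; A Katana2 overlap on the sphere plays a collapse sound, calls AddScore on the Score actor, then destroys the sphere so it cannot trigger again.
; Three seconds after BeginPlay, the actor destroys itself if the procedural mesh is valid.
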(event `self.ReceiveBeginPlay`
  (`KismetSystemLibrary.Delay` 3.0)
  (`/Engine/EditorBlueprintResources/StandardMacros.IsValid` (`self.ProceduralMesh`)
    (:`Is Valid`
      (`self.K2_DestroyActor`))))

(event `self.Sphere.OnComponentBeginOverlap`
  (params (OverlappedComponent :type "PrimitiveComponent Object Reference") (OtherActor :type "Actor Object Reference") (OtherComp :type "PrimitiveComponent Object Reference") (OtherBodyIndex :type Integer) (bFromSweep :type Boolean) (SweepResult :type "HitResult Structure (by ref)"))
  (cast `/Game/Blueprint/Katana2` OtherActor)
  (bind _returnvalue (`GameplayStatics.GetActorOfClass` "/Game/Blueprint/Score.Score_C"))
  (`GameplayStatics.PlaySound2D` "/Game/StarterContent/Audio/Collapse01.Collapse01" 1.0 1.0 0.0 null null)
  (`/Game/Blueprint/Score.Add Score` _returnvalue)
  (`ActorComponent.K2_DestroyComponent` (`self.Sphere`)))

(fn `UserConstructionScript`
  (`KismetProceduralMeshLibrary.CopyProceduralMeshFromStaticMeshComponent` (`self.StaticMesh`) 0 (`self.ProceduralMesh`) true))
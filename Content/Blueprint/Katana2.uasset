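; Katana actor that slices procedural meshes its Plane component overlaps, and can be attached to a given component with physics turned off.
; Each overlap passes a DoOnce, reset on end overlap, then cuts along the plane with a capped second half.
; That half gets physics and a radial impulse, then is destroyed after a short delay.
; BeginPlay also creates and updates a HealthBar widget; detach logic is unconnected.
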(event `self.ReceiveBeginPlay`
  (bind _returnvalue (`|CreateWidget` "/Game/Blueprint/HealthBar.HealthBar_C"))
  (`UserWidget.AddToViewport` _returnvalue 0)
  (set `self.Healthbarreference` _returnvalue)
  (`/Game/Blueprint/HealthBar.UpdateHealthBar` (`self.Healthbarreference`) (`self.health`)))

(event `CustomEvent`
  (params (AttachTo :type "SceneComponent Object Reference"))
  (`PrimitiveComponent.SetSimulatePhysics` (`self.StaticMesh`) false)
  (`SceneComponent.K2_AttachToComponent` (`self.K2_GetRootComponent`) AttachTo "None" "KeepWorld" "KeepWorld" "KeepWorld" false)
  (`SceneComponent.K2_SetRelativeLocationAndRotation` :`self` (`self.StaticMesh`)))

(event `CustomEvent_1`)

(event `self.Plane.OnComponentBeginOverlap`
  (params (OverlappedComponent :type "PrimitiveComponent Object Reference") (OtherActor :type "Actor Object Reference") (OtherComp :type "PrimitiveComponent Object Reference") (OtherBodyIndex :type Integer) (bFromSweep :type Boolean) (SweepResult :type "HitResult Structure (by ref)"))
  (bind _plane (`self.Plane`))
  (bind _returnvalue (`SceneComponent.K2_GetComponentLocation` _plane))
  (`/Engine/EditorBlueprintResources/StandardMacros.DoOnce` false :!label _label
    (:`Completed`
      (bind _asprocedural_mesh_component (cast `ProceduralMeshComponent` OtherComp))
      (bind _outotherhalfprocmesh (`KismetProceduralMeshLibrary.SliceProceduralMesh` _asprocedural_mesh_component _returnvalue (`SceneComponent.GetUpVector` _plane) true "CreateNewSectionForCap"))
      (`PrimitiveComponent.SetSimulatePhysics` _outotherhalfprocmesh true)
      (`PrimitiveComponent.AddRadialImpulse` _outotherhalfprocmesh _returnvalue 50.0 100.0 "RIF_Constant" false)
      (`KismetSystemLibrary.Delay` 1.0)
      (`/Engine/EditorBlueprintResources/StandardMacros.IsValid` _outotherhalfprocmesh
        (:`Is Valid`
          (`ActorComponent.K2_DestroyComponent` _outotherhalfprocmesh))))))

(event `self.Plane.OnComponentEndOverlap`
  (params (OverlappedComponent :type "PrimitiveComponent Object Reference") (OtherActor :type "Actor Object Reference") (OtherComp :type "PrimitiveComponent Object Reference") (OtherBodyIndex :type Integer))
  (goto _label :!via `Reset`))

(fn `UserConstructionScript`)